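; Bolt cutter interaction actor that shows proximity icons to the player and can remove itself from the world.
; Overlap events on the inner and outer icon components toggle their visibility for the player character, swapping outer for inner on closer approach.
; The construction script sizes the inner and outer collision spheres from radius variables.
; A custom event, not called within this Blueprint, destroys the actor after a short delay.
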(event OnComponentBeginOverlap(innerinteracticon)
  (params (OverlappedComponent :type Primitive%20Component%20Object%20Reference) (OtherActor :type Actor%20Object%20Reference) (OtherComp :type Primitive%20Component%20Object%20Reference) (OtherBodyIndex :type Integer) (bFromSweep :type Boolean) (SweepResult :type Hit%20Result%20Structure%20%28by%20ref%29))
  ;[1 1 1] icon
  (if (== OtherActor (Game|GetPlayerCharacter 0))
    (Rendering|SetVisibility (Variables|Default|Getinnerinteracticon) true false)
    (Rendering|SetVisibility (Variables|Default|Getouterinteracticon) false false)))

(event OnComponentEndOverlap(innerinteracticon)
  (params (OverlappedComponent :type Primitive%20Component%20Object%20Reference) (OtherActor :type Actor%20Object%20Reference) (OtherComp :type Primitive%20Component%20Object%20Reference) (OtherBodyIndex :type Integer))
  ;[1 1 1] icon
  (if (== (Game|GetPlayerCharacter 0) OtherActor)
    (Rendering|SetVisibility (Variables|Default|Getinnerinteracticon) false false)
    (Rendering|SetVisibility (Variables|Default|Getouterinteracticon) true false)))

(event OnComponentBeginOverlap(outerinteracticon)
  (params (OverlappedComponent :type Primitive%20Component%20Object%20Reference) (OtherActor :type Actor%20Object%20Reference) (OtherComp :type Primitive%20Component%20Object%20Reference) (OtherBodyIndex :type Integer) (bFromSweep :type Boolean) (SweepResult :type Hit%20Result%20Structure%20%28by%20ref%29))
  ;[1 1 1] icon
  (if (== OtherActor (Game|GetPlayerCharacter 0))
    (Rendering|SetVisibility (Variables|Default|Getouterinteracticon) true false)))

(event OnComponentEndOverlap(outerinteracticon)
  (params (OverlappedComponent :type Primitive%20Component%20Object%20Reference) (OtherActor :type Actor%20Object%20Reference) (OtherComp :type Primitive%20Component%20Object%20Reference) (OtherBodyIndex :type Integer))
  ;[1 1 1] icon
  (if (== (Game|GetPlayerCharacter 0) OtherActor)
    (Rendering|SetVisibility (Variables|Default|Getouterinteracticon) false false)))

(event Custom|CustomEvent
  (Utilities|FlowControl|Delay 0.3)
  (Actor|DestroyActor self))

(fn ConstructionScript
  (Components|Sphere|SetSphereRadius (Variables|Default|Getinnerspherecollision) (Variables|Default|Getinnersphereradius) true)
  (Components|Sphere|SetSphereRadius (Variables|Default|Getouterspherecollision) (Variables|Default|Getoutersphereradius) true))