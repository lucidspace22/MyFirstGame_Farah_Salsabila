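; Base interactable item actor that shows proximity icons to the player and can open an inspection view.
; Two sphere triggers toggle an outer icon at range and swap it for an inner icon up close.
; On Interaction, inspectable items spawn a BP_InspectionItem far off in the world and pass it the mesh, name, description, rotation and scale.
; The construction script applies configurable mesh, icon and radius settings.
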(event OnComponentBeginOverlap(innericonradius)
  (params (OverlappedComponent :type Primitive%20Component%20Object%20Reference) (OtherActor :type Actor%20Object%20Reference) (OtherComp :type Primitive%20Component%20Object%20Reference) (OtherBodyIndex :type Integer) (bFromSweep :type Boolean) (SweepResult :type Hit%20Result%20Structure%20%28by%20ref%29))
  ;[0.8439 0.2554 1] inner n outer icon
  (if (== OtherActor (Game|GetPlayerCharacter 0))
    (Development|SetHiddeninGame (Variables|Default|Getinnericon) false false)
    (Development|SetHiddeninGame (Variables|Default|Getoutericon) true false)))

(event OnComponentEndOverlap(innericonradius)
  (params (OverlappedComponent :type Primitive%20Component%20Object%20Reference) (OtherActor :type Actor%20Object%20Reference) (OtherComp :type Primitive%20Component%20Object%20Reference) (OtherBodyIndex :type Integer))
  ;[0.8439 0.2554 1] inner n outer icon
  (if (== (Game|GetPlayerCharacter 0) OtherActor)
    (Development|SetHiddeninGame (Variables|Default|Getinnericon) true false)
    (Development|SetHiddeninGame (Variables|Default|Getoutericon) false false)))

(event OnComponentBeginOverlap(outericonradius)
  (params (OverlappedComponent :type Primitive%20Component%20Object%20Reference) (OtherActor :type Actor%20Object%20Reference) (OtherComp :type Primitive%20Component%20Object%20Reference) (OtherBodyIndex :type Integer) (bFromSweep :type Boolean) (SweepResult :type Hit%20Result%20Structure%20%28by%20ref%29))
  ;[0.8439 0.2554 1] inner n outer icon
  (if (== OtherActor (Game|GetPlayerCharacter 0))
    (Development|SetHiddeninGame (Variables|Default|Getoutericon) false false)))

(event OnComponentEndOverlap(outericonradius)
  (params (OverlappedComponent :type Primitive%20Component%20Object%20Reference) (OtherActor :type Actor%20Object%20Reference) (OtherComp :type Primitive%20Component%20Object%20Reference) (OtherBodyIndex :type Integer))
  ;[0.8439 0.2554 1] inner n outer icon
  (if (== (Game|GetPlayerCharacter 0) OtherActor)
    (Development|SetHiddeninGame (Variables|Default|Getoutericon) true false)))

(event EventInteraction
  (params (character :type BP%20FPS%20Object%20Reference))
  (if (Variables|Default|GetIs%20Inspectable)
    (bind _returnvalue (Game|SpawnActorfromClass "/Game/01/blueprints/BP_InspectionItem.BP_InspectionItem_C" (Math|Transform|MakeTransform "1000000000.000000,0.000000,0.000000") "Undefined" "MultiplyWithRoot" 0 0))
    (Default|SetItemRotation _returnvalue (Variables|Default|GetInspect%20Item%20Rotation))
    (Default|SetItemScale _returnvalue (Variables|Default|GetInspect%20Item%20Scale))
    (Default|Inspect _returnvalue character (Variables|/Script/Engine.StaticMeshComponent|GetStaticMesh (Variables|Default|GetStaticMesh)) (Variables|Default|GetItem%20Name) (Variables|Default|GetItem%20Description) false)))

(fn ConstructionScript
  (Utilities|FlowControl|Sequence
    (:then_0
      (Components|StaticMesh|SetStaticMesh (Variables|Default|GetStaticMesh) (Variables|Default|GetStatic%20Mesh))
      (Transformation|SetWorldScale3D (Variables|Default|GetStaticMesh) (Math|Conversions|ToVector(Float) (Variables|Default|GetStatic%20Mesh%20Scale)))
      (Transformation|SetRelativeLocation (Variables|Default|GetStaticMesh) (Variables|Default|GetStatic%20Mesh%20Location) false false))
    (:then_1
      (Transformation|SetWorldScale3D (Variables|Default|Getinnericon) (Math|Conversions|ToVector(Float) (Variables|Default|GetInner%20Icon%20Size)))
      (Transformation|SetWorldScale3D (Variables|Default|Getoutericon) (Math|Conversions|ToVector(Float) (Variables|Default|GetOuter%20Icon%20Size)))
      (Transformation|SetRelativeLocation (Variables|Default|Getinnericon) (Variables|Default|GetIcon%20Location) false false))
    (:then_2
      (Components|Sphere|SetSphereRadius (Variables|Default|Getinnericonradius) (Variables|Default|GetInner%20Radius) true)
      (Components|Sphere|SetSphereRadius (Variables|Default|Getoutericonradius) (Variables|Default|GetOuter%20Radius) true))))