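; BP_Door is an interactable swinging door that toggles open and closed, printing "locked" when IsLock is set.
; On Interaction, a timeline plays or reverses to lerp the door's yaw between zero and Degree, while an IsMoving flag blocks retriggering until it finishes.
; IsInverted keeps Degree's sign; otherwise it is forced positive.
; An overlap box only prints a debug message when BP_FPS enters.
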(event OnComponentBeginOverlap(Box)
  (params (OverlappedComponent :type Primitive%20Component%20Object%20Reference) (OtherActor :type Actor%20Object%20Reference) (OtherComp :type Primitive%20Component%20Object%20Reference) (OtherBodyIndex :type Integer) (bFromSweep :type Boolean) (SweepResult :type Hit%20Result%20Structure%20%28by%20ref%29))
  (Utilities|Casting|CastToBP_FPS OtherActor)
  (Development|PrintString "MASOK"))

(event EventInteraction
  (if (Variables|Default|GetIsInverted)
    (Variables|Default|SetDegree (Variables|Default|GetDegree))
    (else
      (Variables|Default|SetDegree (Math|Float|Absolute(Float) (Variables|Default|GetDegree)))))
  (if (Variables|Default|GetIsLock)
    (Development|PrintString "locked")
    (elif (not (Variables|Default|GetIsMoving))
      (Variables|Default|SetIsMoving true)
      (bind _output_get (Variables|Default|SetIsOpened (not (Variables|Default|GetIsOpened))))
      (if _output_get
        (bind _door_alpha (Timeline|TL_Doors Play)
          (:Update
            (Transformation|SetRelativeRotation (Variables|Default|GetDoor) (Math|Rotator|MakeRotator 0.0 0.0 (Math|Float|Lerp 0.0 (Variables|Default|GetDegree) _door_alpha)) false false))
          (:Finished
            (Variables|Default|SetIsMoving false)))
        (else
          (Timeline|TL_Doors Reverse))))))

(fn ConstructionScript)