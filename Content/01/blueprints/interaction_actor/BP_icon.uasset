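; BP_icon is an interaction prompt actor that swaps two icons based on the player's proximity.
; Overlap events on the inner and outer icon components, filtered to BP_FPS, toggle visibility, with the inner icon replacing the outer one.
; Most toggles also depend on an IsOverlappingActor check on the player.
; The construction script sizes separate inner and outer collision spheres from radius variables.
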(event OnComponentBeginOverlap(innerinteracticon)
  (params (OverlappedComponent :type Primitive%20Component%20Object%20Reference) (OtherActor :type Actor%20Object%20Reference) (OtherComp :type Primitive%20Component%20Object%20Reference) (OtherBodyIndex :type Integer) (bFromSweep :type Boolean) (SweepResult :type Hit%20Result%20Structure%20%28by%20ref%29))
  (bind _asbp_fps (Utilities|Casting|CastToBP_FPS OtherActor))
  (if true
    (Rendering|SetVisibility (Variables|Default|Getinnerinteracticon) true false)
    (Rendering|SetVisibility (Variables|Default|Getouterinteracticon) false false)))

(event OnComponentEndOverlap(innerinteracticon)
  (params (OverlappedComponent :type Primitive%20Component%20Object%20Reference) (OtherActor :type Actor%20Object%20Reference) (OtherComp :type Primitive%20Component%20Object%20Reference) (OtherBodyIndex :type Integer))
  (bind _asbp_fps (Utilities|Casting|CastToBP_FPS OtherActor))
  (if (not (Collision|IsOverlappingActor _asbp_fps 0 :!class /Script/Engine.Actor))
    (Rendering|SetVisibility (Variables|Default|Getinnerinteracticon) false false)
    (Rendering|SetVisibility (Variables|Default|Getouterinteracticon) true false)))

(event OnComponentBeginOverlap(outerinteracticon)
  (params (OverlappedComponent :type Primitive%20Component%20Object%20Reference) (OtherActor :type Actor%20Object%20Reference) (OtherComp :type Primitive%20Component%20Object%20Reference) (OtherBodyIndex :type Integer) (bFromSweep :type Boolean) (SweepResult :type Hit%20Result%20Structure%20%28by%20ref%29))
  (bind _asbp_fps (Utilities|Casting|CastToBP_FPS OtherActor))
  (if (Collision|IsOverlappingActor _asbp_fps 0 :!class /Script/Engine.Actor)
    (Rendering|SetVisibility (Variables|Default|Getouterinteracticon) true false)))

(event OnComponentEndOverlap(outerinteracticon)
  (params (OverlappedComponent :type Primitive%20Component%20Object%20Reference) (OtherActor :type Actor%20Object%20Reference) (OtherComp :type Primitive%20Component%20Object%20Reference) (OtherBodyIndex :type Integer))
  (bind _asbp_fps (Utilities|Casting|CastToBP_FPS OtherActor))
  (if (not (Collision|IsOverlappingActor _asbp_fps 0 :!class /Script/Engine.Actor))
    (Rendering|SetVisibility (Variables|Default|Getouterinteracticon) false false)))

(fn ConstructionScript
  (Components|Sphere|SetSphereRadius (Variables|Default|Getinnerspherecollision) (Variables|public|Getinnersphereradius) true)
  (Components|Sphere|SetSphereRadius (Variables|Default|Getouterspherecollision) (Variables|public|Getoutersphereradius) true))